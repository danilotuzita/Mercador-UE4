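; Player character with arrow-relative movement, controller yaw and a spring-arm camera with limited pitch and zoom, built for talking to NPCs.
; An interaction-radius overlap tracks one nearby Bp_MasterNPC, notifies it on entering or leaving view, and E interacts with it.
; It spawns a BP_DialogueManager on BeginPlay and feeds it number, arrow and continue input, with timers repeating held arrows.
; Dialogue-finished and decision events are forwarded to that NPC.
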(event OnComponentBeginOverlap(InteractRadius)
  (params (OverlappedComponent :type Primitive%20Component%20Object%20Reference) (OtherActor :type Actor%20Object%20Reference) (OtherComp :type Primitive%20Component%20Object%20Reference) (OtherBodyIndex :type Integer) (bFromSweep :type Boolean) (SweepResult :type Hit%20Result%20Structure%20%28by%20ref%29))
  (bind _asbp_master_npc (Utilities|Casting|CastToBp_MasterNPC OtherActor))
  (Utilities|IsValid (Variables|Default|GetNearbyNPC)
    (:Is%20Valid
      (Default|OnLeavePlayerView (Variables|Default|GetNearbyNPC)))
    (:Is%20Not%20Valid
      _))
  (bind _output_get (Variables|Default|SetNearbyNPC _asbp_master_npc))
  (Default|OnEnterPlayerView _output_get))

(event OnComponentEndOverlap(InteractRadius)
  (params (OverlappedComponent :type Primitive%20Component%20Object%20Reference) (OtherActor :type Actor%20Object%20Reference) (OtherComp :type Primitive%20Component%20Object%20Reference) (OtherBodyIndex :type Integer))
  (if (== OtherActor (Variables|Default|GetNearbyNPC))
    (Default|OnLeavePlayerView (Variables|Default|GetNearbyNPC))
    (Variables|Default|SetNearbyNPC 0)))

(event Custom|OnDialogueFinished
  (params (Index :type Integer))
  ;[1 1 1] On DialogueFinnished
  (Utilities|IsValid (Variables|Default|GetNearbyNPC)
    (:Is%20Valid
      (Default|OnDialogueEnd (Variables|Default|GetNearbyNPC) Index))))

(event Custom|OnDecisionMade
  (params (DecisionIndex :type Integer) (OptionIndex :type Integer))
  (bind _nearbynpc (Variables|Default|GetNearbyNPC))
  ;[1 1 1] On DecisionMade
  (Utilities|IsValid _nearbynpc
    (:Is%20Valid
      (Default|OnDecisionMade _nearbynpc DecisionIndex OptionIndex))))

(event Custom|UpKeyTimerEvent
  ;[1 1 1] Up and Down Keys
  (Default|HandleUpKey (Variables|Default|GetDialogManager)))

(event Custom|DownKeyTimerEvent
  ;[1 1 1] Up and Down Keys
  (Default|HandleDownKey (Variables|Default|GetDialogManager)))

(event EventBeginPlay
  ;[1 1 1] Begin Play
  (bind _returnvalue (Game|SpawnActorfromClass "/Game/DialogueSystem/Blueprints/BP_DialogueManager.BP_DialogueManager_C" (Math|Transform|MakeTransform "0, 0, 0" "0, 0, 0" "1,1,1") "AlwaysSpawn" 0 self 0))
  (Variables|Default|SetDialogManager _returnvalue))

(event Input|ActionEvents|InputActionZooming
  (params (Key :type Key%20Structure :default "AnyKey"))
  (bind _springarm (Variables|Default|GetSpringArm))
  ;[1 1 1] Zooming
  (:Pressed
    (bind _output_get (Variables|Default|SetArmLenght (Variables|/Script/Engine.SpringArmComponent|GetTargetArmLength (Variables|Default|GetSpringArm))))
    (if (> _output_get 5e+02)
      (Variables|/Script/Engine.SpringArmComponent|SetTargetArmLength _springarm (- (Variables|Default|GetArmLenght) 1e+02))
      (Variables|Default|SetArmLenght (Variables|/Script/Engine.SpringArmComponent|GetTargetArmLength _springarm)))))

(event Input|ActionEvents|InputActionContinue
  (params (Key :type Key%20Structure :default "AnyKey"))
  ;[1 1 1] Continue Command
  (:Pressed
    (Default|HandleContinueCommand (Variables|Default|GetDialogManager))))

(event Input|ActionEvents|InputActionUnzooming
  (params (Key :type Key%20Structure :default "AnyKey"))
  (bind _springarm (Variables|Default|GetSpringArm))
  ;[1 1 1] Zooming
  (:Pressed
    (bind _output_get (Variables|Default|SetArmLenght (Variables|/Script/Engine.SpringArmComponent|GetTargetArmLength (Variables|Default|GetSpringArm))))
    (if (< _output_get 1.2e+03)
      (Variables|/Script/Engine.SpringArmComponent|SetTargetArmLength _springarm (+ (Variables|Default|GetArmLenght) 1e+02))
      (Variables|Default|SetArmLenght (Variables|/Script/Engine.SpringArmComponent|GetTargetArmLength _springarm)))))

(event Input|ActionEvents|InputActionPitchUp
  (params (Key :type Key%20Structure :default "AnyKey"))
  ;[1 1 1] Pitch
  ;;[1 1 1] Wheel
  (:Pressed
    (if (< (.Pitch (Math|Rotator|BreakRotator (Transformation|GetWorldRotation (Variables|Default|GetSpringArm)))) 5.0)
      (Transformation|AddLocalRotation (Variables|Default|GetSpringArm) "10.000000, 0, 0" false false))))

(event Input|ActionEvents|InputActionPitchDown
  (params (Key :type Key%20Structure :default "AnyKey"))
  ;[1 1 1] Pitch
  ;;[1 1 1] Wheel
  (:Pressed
    (if (> (.Pitch (Math|Rotator|BreakRotator (Transformation|GetWorldRotation (Variables|Default|GetSpringArm)))) -8e+01)
      (Transformation|AddLocalRotation (Variables|Default|GetSpringArm) "-10.000000, 0, 0" false false))))

(event Input|AxisEvents|InputAxisMoveForward
  (params (AxisValue :type Float%20%28single-precision%29))
  ;[1 1 1] Movement
  (Pawn|Input|AddMovementInput (Math|Vector|GetForwardVector (Variables|Default|GetArrowComponent)) AxisValue false))

(event Input|AxisEvents|InputAxisRotation
  (params (AxisValue :type Float%20%28single-precision%29))
  ;[1 1 1] Movement
  (Pawn|Input|AddControllerYawInput AxisValue))

(event Input|AxisEvents|InputAxisMousePitch
  (params (AxisValue :type Float%20%28single-precision%29))
  (bind _springarm (Variables|Default|GetSpringArm))
  (bind _returnvalue (Transformation|GetWorldRotation _springarm))
  (bind _pitch (Math|Rotator|BreakRotator _returnvalue))
  ;[1 1 1] Pitch
  ;;[1 1 1] Mouse
  (if (>= AxisValue 0.0)
    (if (< _pitch 5.0)
      (Transformation|AddLocalRotation _springarm (Math|Rotator|MakeRotator 0.0 AxisValue 0.0) false false :!label _label))
    (elif (> _pitch -8e+01)
      (goto _label))))

(event Input|AxisEvents|InputAxisMoveRight
  (params (AxisValue :type Float%20%28single-precision%29))
  ;[1 1 1] Movement
  (Pawn|Input|AddMovementInput (Math|Vector|GetRightVector (Variables|Default|GetArrowComponent)) AxisValue false))

(event Input|KeyboardEvents|Down
  (params (Key :type Key%20Structure :default "AnyKey"))
  ;[1 1 1] Up and Down Keys
  (:Pressed
    (Variables|Default|SetDownDown? true)
    (bind _handled_ (Default|HandleDownKey (Variables|Default|GetDialogManager)))
    (if _handled_
      (bind _returnvalue (Utilities|Time|SetTimerbyEvent (delegate Custom|DownKeyTimerEvent) 0.2 true))))
  (:Released
    (Variables|Default|SetDownDown? false)
    (Utilities|Time|ClearandInvalidateTimerbyHandle _returnvalue)))

(event Input|KeyboardEvents|Up
  (params (Key :type Key%20Structure :default "AnyKey"))
  ;[1 1 1] Up and Down Keys
  (:Pressed
    (Variables|Default|SetUpDown? true)
    (bind _handled_ (Default|HandleUpKey (Variables|Default|GetDialogManager)))
    (if _handled_
      (bind _returnvalue (Utilities|Time|SetTimerbyEvent (delegate Custom|UpKeyTimerEvent) 0.2 true))))
  (:Released
    (Variables|Default|SetUpDown? false)
    (Utilities|Time|ClearandInvalidateTimerbyHandle _returnvalue)))

(event Input|KeyboardEvents|E
  (params (Key :type Key%20Structure :default "AnyKey"))
  (bind _nearbynpc (Variables|Default|GetNearbyNPC))
  (:Pressed
    (Utilities|IsValid _nearbynpc
      (:Is%20Valid
        (Default|OnInteract _nearbynpc self)))))

(event Input|KeyboardEvents|1
  (params (Key :type Key%20Structure :default "AnyKey"))
  (bind _dialogmanager (Variables|Default|GetDialogManager))
  ;[1 1 1] Number Keys
  (:Pressed
    (Variables|Default|SetPressedNumber 1)
    (Utilities|IsValid _dialogmanager
      (:Is%20Valid
        (Default|HandleNumberKey _dialogmanager (Variables|Default|GetPressedNumber))))))

(event Input|KeyboardEvents|2
  (params (Key :type Key%20Structure :default "AnyKey"))
  (bind _dialogmanager (Variables|Default|GetDialogManager))
  ;[1 1 1] Number Keys
  (:Pressed
    (Variables|Default|SetPressedNumber 2)
    (Utilities|IsValid _dialogmanager
      (:Is%20Valid
        (Default|HandleNumberKey _dialogmanager (Variables|Default|GetPressedNumber))))))

(event Input|KeyboardEvents|3
  (params (Key :type Key%20Structure :default "AnyKey"))
  (bind _dialogmanager (Variables|Default|GetDialogManager))
  ;[1 1 1] Number Keys
  (:Pressed
    (Variables|Default|SetPressedNumber 3)
    (Utilities|IsValid _dialogmanager
      (:Is%20Valid
        (Default|HandleNumberKey _dialogmanager (Variables|Default|GetPressedNumber))))))

(event Input|KeyboardEvents|4
  (params (Key :type Key%20Structure :default "AnyKey"))
  (bind _dialogmanager (Variables|Default|GetDialogManager))
  ;[1 1 1] Number Keys
  (:Pressed
    (Variables|Default|SetPressedNumber 4)
    (Utilities|IsValid _dialogmanager
      (:Is%20Valid
        (Default|HandleNumberKey _dialogmanager (Variables|Default|GetPressedNumber))))))

(event Input|KeyboardEvents|5
  (params (Key :type Key%20Structure :default "AnyKey"))
  (bind _dialogmanager (Variables|Default|GetDialogManager))
  ;[1 1 1] Number Keys
  (:Pressed
    (Variables|Default|SetPressedNumber 5)
    (Utilities|IsValid _dialogmanager
      (:Is%20Valid
        (Default|HandleNumberKey _dialogmanager (Variables|Default|GetPressedNumber))))))

(event Input|KeyboardEvents|6
  (params (Key :type Key%20Structure :default "AnyKey"))
  (bind _dialogmanager (Variables|Default|GetDialogManager))
  ;[1 1 1] Number Keys
  (:Pressed
    (Variables|Default|SetPressedNumber 6)
    (Utilities|IsValid _dialogmanager
      (:Is%20Valid
        (Default|HandleNumberKey _dialogmanager (Variables|Default|GetPressedNumber))))))

(event Input|KeyboardEvents|7
  (params (Key :type Key%20Structure :default "AnyKey"))
  (bind _dialogmanager (Variables|Default|GetDialogManager))
  ;[1 1 1] Number Keys
  (:Pressed
    (Variables|Default|SetPressedNumber 7)
    (Utilities|IsValid _dialogmanager
      (:Is%20Valid
        (Default|HandleNumberKey _dialogmanager (Variables|Default|GetPressedNumber))))))

(fn ConstructionScript)