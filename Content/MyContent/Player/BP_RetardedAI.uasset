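; BP_RetardedAI is an NPC that shows a randomly chosen name to the player when nearby.
; On BeginPlay it picks one name from a hardcoded list and writes it to a text render component.
; Overlapping its ActionCollision with BP_PlayerCharacter shows the text and passes the name to the player as the overlapped NPC.
; Ending the overlap hides the text and clears that name on the player.
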(event OnComponentBeginOverlap(ActionCollision)
  (params (OverlappedComponent :type Primitive%20Component%20Object%20Reference) (OtherActor :type Actor%20Object%20Reference) (OtherComp :type Primitive%20Component%20Object%20Reference) (OtherBodyIndex :type Integer) (bFromSweep :type Boolean) (SweepResult :type Hit%20Result%20Structure%20%28by%20ref%29))
  (bind _asbp_player_character (Utilities|Casting|CastToBP_PlayerCharacter OtherActor))
  (Rendering|SetVisibility (Variables|Default|GetTextRender) true false)
  (Default|SetOverlapingNPCName _asbp_player_character (Variables|Default|GetName)))

(event OnComponentEndOverlap(ActionCollision)
  (params (OverlappedComponent :type Primitive%20Component%20Object%20Reference) (OtherActor :type Actor%20Object%20Reference) (OtherComp :type Primitive%20Component%20Object%20Reference) (OtherBodyIndex :type Integer))
  (bind _asbp_player_character (Utilities|Casting|CastToBP_PlayerCharacter OtherActor))
  (Rendering|SetVisibility (Variables|Default|GetTextRender) false false)
  (Default|SetOverlapingNPCName _asbp_player_character))

(event EventBeginPlay
  (bind _output_get (Variables|Default|SetName (Utilities|String|ToString(Text) (Utilities|Array|Get(acopy) (Utilities|Array|MakeArray (Utilities|Text|ToText(String) "João") (Utilities|Text|ToText(String) "Maria") (Utilities|Text|ToText(String) "Astolfo") (Utilities|Text|ToText(String) "Leo") (Utilities|Text|ToText(String) "Serafim") (Utilities|Text|ToText(String) "Monkey")) (Math|Random|RandomIntegerinRange 0 5)))))
  (Rendering|Components|TextRender|SetText (Variables|Default|GetTextRender) (Utilities|Text|ToText(String) _output_get)))

(fn ConstructionScript)