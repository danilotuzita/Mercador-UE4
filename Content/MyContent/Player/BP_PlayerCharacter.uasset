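; Player character Blueprint with arrow-relative movement, controller yaw turning, range-checked spring-arm zoom and pitch, and simple NPC dialogue.
; A hidden Conversation widget is created on BeginPlay; pressing E with an overlapping NPC name set fills and shows it, enables the cursor and disables input.
; SetOption stores the validated choice, and SelectOption calls ChangeMessage to display the matching hardcoded reply.
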(event Custom|SelectOption
  (CallFunction|ChangeMessage "Sorry, what?" "Nice to meet you too" "-" true "Bye!" false "" false))

(event EventBeginPlay
  ;[1 1 1] HUD
  (bind _returnvalue (UserInterface|CreateWidget "/Game/MyContent/Player/HUD/Conversation.Conversation_C" (Game|GetPlayerController 0)))
  (bind _output_get (Variables|Default|SetHUDRef _returnvalue))
  (UserInterface|Viewport|AddtoViewport _output_get 0)
  (Widget|SetVisibility (Variables|Default|GetHUDRef) "Hidden"))

(event Input|ActionEvents|InputActionZooming
  (params (Key :type Key%20Structure :default "AnyKey"))
  (bind _springarm (Variables|Default|GetSpringArm))
  ;[1 1 1] Zooming
  (:Pressed
    (bind _output_get (Variables|Default|SetArmLenght (Variables|/Script/Engine.SpringArmComponent|GetTargetArmLength (Variables|Default|GetSpringArm))))
    (if (> _output_get 5e+02)
      (Variables|/Script/Engine.SpringArmComponent|SetTargetArmLength _springarm (- (Variables|Default|GetArmLenght) 1e+02))
      (Variables|Default|SetArmLenght (Variables|/Script/Engine.SpringArmComponent|GetTargetArmLength _springarm)))))

(event Input|ActionEvents|InputActionUnzooming
  (params (Key :type Key%20Structure :default "AnyKey"))
  (bind _springarm (Variables|Default|GetSpringArm))
  ;[1 1 1] Zooming
  (:Pressed
    (bind _output_get (Variables|Default|SetArmLenght (Variables|/Script/Engine.SpringArmComponent|GetTargetArmLength (Variables|Default|GetSpringArm))))
    (if (< _output_get 1.2e+03)
      (Variables|/Script/Engine.SpringArmComponent|SetTargetArmLength _springarm (+ (Variables|Default|GetArmLenght) 1e+02))
      (Variables|Default|SetArmLenght (Variables|/Script/Engine.SpringArmComponent|GetTargetArmLength _springarm)))))

(event Input|ActionEvents|InputActionPitchUp
  (params (Key :type Key%20Structure :default "AnyKey"))
  ;[1 1 1] Pitch
  ;;[1 1 1] Wheel
  (:Pressed
    (if (< (.Pitch (Math|Rotator|BreakRotator (Transformation|GetWorldRotation (Variables|Default|GetSpringArm)))) -2e+01)
      (Transformation|AddLocalRotation (Variables|Default|GetSpringArm) "10.000000, 0, 0" false false))))

(event Input|ActionEvents|InputActionPitchDown
  (params (Key :type Key%20Structure :default "AnyKey"))
  ;[1 1 1] Pitch
  ;;[1 1 1] Wheel
  (:Pressed
    (if (> (.Pitch (Math|Rotator|BreakRotator (Transformation|GetWorldRotation (Variables|Default|GetSpringArm)))) -8e+01)
      (Transformation|AddLocalRotation (Variables|Default|GetSpringArm) "-10.000000, 0, 0" false false))))

(event Input|AxisEvents|InputAxisMoveForward
  (params (AxisValue :type Float%20%28single-precision%29))
  ;[1 1 1] Movement
  (Pawn|Input|AddMovementInput (Math|Vector|GetForwardVector (Variables|Default|GetArrowComponent)) AxisValue false))

(event Input|AxisEvents|InputAxisRotation
  (params (AxisValue :type Float%20%28single-precision%29))
  ;[1 1 1] Movement
  (Pawn|Input|AddControllerYawInput AxisValue))

(event Input|AxisEvents|InputAxisMousePitch
  (params (AxisValue :type Float%20%28single-precision%29))
  (bind _springarm (Variables|Default|GetSpringArm))
  (bind _returnvalue (Transformation|GetWorldRotation _springarm))
  (bind _pitch (Math|Rotator|BreakRotator _returnvalue))
  ;[1 1 1] Pitch
  ;;[1 1 1] Mouse
  (if (>= AxisValue 0.0)
    (if (< _pitch -2e+01)
      (Transformation|AddLocalRotation _springarm (Math|Rotator|MakeRotator 0.0 AxisValue 0.0) false false :!label _label))
    (elif (> _pitch -8e+01)
      (goto _label))))

(event Input|AxisEvents|InputAxisMoveRight
  (params (AxisValue :type Float%20%28single-precision%29))
  ;[1 1 1] Movement
  (Pawn|Input|AddMovementInput (Math|Vector|GetRightVector (Variables|Default|GetArrowComponent)) AxisValue false))

(event Input|KeyboardEvents|E
  (params (Key :type Key%20Structure :default "AnyKey"))
  (bind _returnvalue (Game|GetPlayerController 0))
  (bind _hudref (Variables|Default|GetHUDRef))
  (bind _overlapingnpcname (Variables|Default|GetOverlapingNPCName))
  (:Pressed
    (if (Utilities|Enum|NotEqual(Enum) (Variables|Default|GetOverlapingNPCName) "")
      (Default|ElementVisibility _hudref true true false)
      (Default|SetText _hudref _overlapingnpcname (Utilities|Text|ToText(String) (Utilities|String|Append "Hello there, I'm " _overlapingnpcname)) "Yeah, I know. Just saw above your head." "Hello! Nice to meet you.")
      (Widget|SetVisibility (Variables|Default|GetHUDRef) "Visible")
      (Variables|/Script/Engine.PlayerController|SetbShowMouseCursor _returnvalue true)
      (Input|DisableInput _returnvalue))))

(fn ConstructionScript)

(fn SetOverlapingNPCName
  (params (whoIsTalking :type String))
  (Variables|Default|SetOverlapingNPCName whoIsTalking))

(fn SetOption
  (params (Op :type Integer))
  (if (and (>= Op 0) (<= Op 2))
    (Variables|Default|SetChosenOption Op)
    (else
      (Development|PrintString "Error Setting Option" true true "(R=1.000000,G=0.029601,B=0.000000,A=1.000000)" 99.0)
      (Variables|Default|SetChosenOption -1))))

(fn ChangeMessage
  (params (NewMessage0 :type Text) (NewMessage1 :type Text) (NewMessage2 :type Text) (Button0 :type Boolean) (Option0 :type String) (Button1 :type Boolean) (Option1 :type String) (Button2 :type Boolean) (Option2 :type String))
  (if (!= (Variables|Default|GetChosenOption) -1)
    (Default|ElementVisibility (Variables|Default|GetHUDRef) Button0 Button1 Button2)
    (if (== (Variables|Default|GetChosenOption) 0)
      (Variables|Default|SetMessage NewMessage0)
      (elif (== (Variables|Default|GetChosenOption) 1)
        (Variables|Default|SetMessage NewMessage1)
        (elif (== (Variables|Default|GetChosenOption) 2)
          (Variables|Default|SetMessage NewMessage2)
          (else
            (Variables|Default|SetMessage "")))))
    (Default|SetText (Variables|Default|GetHUDRef) (Variables|Default|GetOverlapingNPCName) (Variables|Default|GetMessage) Option0 Option1 Option2)))